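; Player chicken character for a Crossy Road-style game, hopping in four directions to dodge traffic and collect coins.
; Arrow keys jump and rotate the mesh, and OnJumped launches it along the direction flag, defaulting to left.
; Overlap casts handle vehicle and train deaths, drowning activation, coin pickups and level scoring.
; Deaths play sound and visual feedback before a delayed destroy, and Destroyed restarts through the CrossyRoad game mode.
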(event `self.ReceiveTick`
  (params (DeltaSeconds :type "Float (single-precision)")))

(event `self.OnJumped`
  (`GameplayStatics.PlaySoundAtLocation` "/Game/CR/Sounds/ChickenSquak.ChickenSquak" (`self.K2_GetActorLocation`) (struct) 1.0 1.0 0.0 null null null)
  (if (`NavMovementComponent.IsMovingOnGround` (`self.CharacterMovement`))
    _
    (elif (`self.Forward`)
      (`self.LaunchCharacter` (100.0 0.0 0.0))
      (set `self.Forward` false)
      (elif (`self.Backward`)
        (`self.LaunchCharacter` (-100.0 0.0 0.0))
        (set `self.Backward` false)
        (elif (`self.Right`)
          (`self.LaunchCharacter` (0.0 100.0 0.0))
          (set `self.Right` false)
          (else
            (`self.LaunchCharacter` (0.0 -100.0 0.0))))))))

(event `Key|Left`
  (params (Key :type "Key Structure"))
  (:`Pressed`
    (`self.Jump`)
    (`SceneComponent.K2_SetRelativeRotation` :`self` (`self.Chicken`))))

(event `Key|Right`
  (params (Key :type "Key Structure"))
  (:`Pressed`
    (`self.Jump`)
    (`SceneComponent.K2_SetRelativeRotation` (`self.Chicken`) (struct :`Yaw` 180.0) false false)
    (set `self.Right` true)))

(event `Key|Up`
  (params (Key :type "Key Structure"))
  (:`Pressed`
    (`self.Jump`)
    (`SceneComponent.K2_SetRelativeRotation` (`self.Chicken`) (struct :`Yaw` 90.0) false false)
    (set `self.Forward` true)))

(event `Key|Down`
  (params (Key :type "Key Structure"))
  (:`Pressed`
    (`self.Jump`)
    (`SceneComponent.K2_SetRelativeRotation` (`self.Chicken`) (struct :`Yaw` 270.0) false false)
    (set `self.Backward` true)))

(event `self.ReceiveActorBeginOverlap`
  (params (OtherActor :type "Actor Object Reference"))
  (bind _returnvalue (`self.K2_GetActorLocation`))
  (cast `/Game/CR/Blueprints/RedTruck` OtherActor
    (:`then`
      (`StaticMeshComponent.SetStaticMesh` (`self.Chicken`) "/Game/CR/Meshes/squashed.squashed")
      (`GameplayStatics.PlaySoundAtLocation` "/Game/CR/Sounds/ChickenDeath.ChickenDeath" _returnvalue (struct) 1.0 1.0 0.0 null null null :!label _label)
      (`KismetSystemLibrary.Delay` 0.8)
      (`self.K2_DestroyActor` :!label _label_2))
    (:`CastFailed`
      (cast `/Game/CR/Blueprints/Train` OtherActor
        (:`then`
          (`ActorComponent.Activate` (`self.ChickenCollision`) true)
          (`SceneComponent.SetVisibility` (`self.Chicken`) false false)
          (`GameplayStatics.PlaySoundAtLocation` "/Game/CR/Sounds/ChickenDeath.ChickenDeath" _returnvalue (struct) 1.0 1.0 0.0 null null null)
          (`KismetSystemLibrary.Delay` 1.3)
          (goto _label_2))
        (:`CastFailed`
          (cast `/Game/CR/Blueprints/BlueCar` OtherActor
            (:`then`
              (`StaticMeshComponent.SetStaticMesh` (`self.Chicken`) "/Game/CR/Meshes/squashedz.squashedz" :!label _label_3)
              (goto _label))
            (:`CastFailed`
              (cast `/Game/CR/Blueprints/GreenCar` OtherActor
                (:`then`
                  (goto _label_3))
                (:`CastFailed`
                  (cast `/Game/CR/Blueprints/WaterCollision` OtherActor
                    (:`then`
                      (`ActorComponent.Activate` (`self.ChickenDrowning`) true))
                    (:`CastFailed`
                      (bind _ascoin (cast `/Game/Blueprints/coin` OtherActor)
                        (:`then`
                          (bind _output_get (set `self.CoinScore` (+ (`self.CoinScore`) (`self.CoinIncrease`))))
                          (`self.K2_DestroyActor` _ascoin)
                          (`KismetSystemLibrary.PrintText` (`KismetTextLibrary.Conv_IntToText` _output_get)))
                        (:`CastFailed`
                          (cast `/Game/CR/Blueprints/BP_Level` OtherActor)
                          (bind _output_get_2 (set `self.Score` (+ (`self.Score`) (`self.ScoreIncrease`))))
                          (`KismetSystemLibrary.PrintText` (`KismetTextLibrary.Conv_IntToText` _output_get_2)))))))))))))))

(event `self.ReceiveDestroyed`
  (bind _ascrossy_road (cast `/Game/CR/Blueprints/CrossyRoad` (`GameplayStatics.GetGameMode`)))
  (`GameMode.RestartGame` _ascrossy_road))

(fn `UserConstructionScript`)