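; GreenCar is a car actor that drives itself repeatedly along a track's spline when Active at BeginPlay.
; MoveCar plays the CarMovement timeline at a rate set by a random lap duration, starting from StartOffset.
; Each update maps the timeline's Alpha to spline distance and sets the car's world location and rotation.
; On finish, it calls MoveCar again with a new random duration, restarting from StartOffset.
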(event `self.ReceiveBeginPlay`
  (if (`self.Active`)
    (set `self.CarSpeed` (`KismetMathLibrary.RandomFloatInRange` 3.0 5.0) :!label _label)
    (`self.MoveCar` (`self.&Track`))))

(event `MoveCar`
  (params (TrackRef :type "/Game/CR/Blueprints/Track Object Reference"))
  (bind _returnvalue (`KismetMathLibrary.Lerp` 0.0 (`SplineComponent.GetSplineLength` (`/Game/CR/Blueprints/Track.Spline` (`self.&Track`))) (`self.Alpha`)))
  (set `self.&Track` TrackRef)
  (set `self.CarSpeed` (`KismetMathLibrary.RandomFloatInRange` 3.0 5.0))
  (`TimelineComponent.SetPlayRate` (`self.CarMovement`) (/ 1.0 (`self.CarSpeed`)))
  (`TimelineComponent.SetNewTime` (`self.CarMovement`) (`self.StartOffset`))
  (bind (_direction _alpha) (`Timeline|CarMovement`)
    (:`Update`
      (set `self.Alpha` _alpha)
      (`self.K2_SetActorLocationAndRotation` (`SplineComponent.GetLocationAtDistanceAlongSpline` (`/Game/CR/Blueprints/Track.Spline` (`self.&Track`)) _returnvalue "World") (`SplineComponent.GetRotationAtDistanceAlongSpline` (`/Game/CR/Blueprints/Track.Spline` (`self.&Track`)) _returnvalue "World")))
    (:`Finished`
      (goto _label))))

(fn `UserConstructionScript`)