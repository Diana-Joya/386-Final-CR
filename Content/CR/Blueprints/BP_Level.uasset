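; BP_Level is one terrain row in a Crossy Road-style chicken game, starting as random grass.
; SetMesh randomizes it into grass with trees, coins and rocks, road, train tracks, or water with lilypads or logs.
; Vehicles and logs receive spawned Track actors through MoveCar.
; A chicken entering TriggerZone makes LevelSpawner spawn another level, while two side boxes call StopJumping on it.
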(event `self.ReceiveBeginPlay`
  (`self.SetInitialMesh`))

(event `self.TriggerZone.OnComponentBeginOverlap`
  (params (OverlappedComponent :type "PrimitiveComponent Object Reference") (OtherActor :type "Actor Object Reference") (OtherComp :type "PrimitiveComponent Object Reference") (OtherBodyIndex :type Integer) (bFromSweep :type Boolean) (SweepResult :type "HitResult Structure (by ref)"))
  (bind _levelspawner (`self.LevelSpawner`))
  (cast `/Game/CR/Blueprints/Chicken` OtherActor)
  (`/Engine/EditorBlueprintResources/StandardMacros.IsValid` "/Game/CR/Blueprints/Chicken.Chicken"
    (:`Is Valid`
      (`/Game/CR/Blueprints/BP_LevelSpawner.SpawnLevelAtSpawnPoint` _levelspawner))
    (:`Is Not Valid`
      (`/Game/CR/Blueprints/BP_LevelSpawner.SpawnInitialLevels` _levelspawner)
      (`self.K2_DestroyActor`))))

(event `self.Box.OnComponentBeginOverlap`
  (params (OverlappedComponent :type "PrimitiveComponent Object Reference") (OtherActor :type "Actor Object Reference") (OtherComp :type "PrimitiveComponent Object Reference") (OtherBodyIndex :type Integer) (bFromSweep :type Boolean) (SweepResult :type "HitResult Structure (by ref)"))
  (bind _aschicken (cast `/Game/CR/Blueprints/Chicken` OtherActor))
  (`Character.StopJumping` _aschicken))

(event `self.Box1.OnComponentBeginOverlap`
  (params (OverlappedComponent :type "PrimitiveComponent Object Reference") (OtherActor :type "Actor Object Reference") (OtherComp :type "PrimitiveComponent Object Reference") (OtherBodyIndex :type Integer) (bFromSweep :type Boolean) (SweepResult :type "HitResult Structure (by ref)"))
  (bind _aschicken (cast `/Game/CR/Blueprints/Chicken` OtherActor))
  (`Character.StopJumping` _aschicken))

(fn `SetInitialMesh`
  (switch `int` (`KismetMathLibrary.RandomIntegerInRange` 0 1)
    (:`0`
      (`StaticMeshComponent.SetStaticMesh` (`self.StaticMesh`) "/Game/CR/Meshes/brightgrass.brightgrass"))
    (:`1`
      (`StaticMeshComponent.SetStaticMesh` (`self.StaticMesh`) "/Game/CR/Meshes/lightgrass.lightgrass"))))

(fn `SetMesh`
  (bind (_dynspawn_x _dynspawn_y) (`KismetMathLibrary.BreakVector` (`self.DynSpawn`)))
  (bind (_dynspawn_x_2 _dynspawn_y_2) (`KismetMathLibrary.BreakVector` (`self.DynSpawn`)))
  (bind _returnvalue (+ (`SceneComponent.K2_GetComponentLocation` (`self.StaticMesh`)) (0.0 1050.0 0.0)))
  (bind _returnvalue_2 (+ (`SceneComponent.K2_GetComponentLocation` (`self.StaticMesh`)) (0.0 1050.0 0.0)))
  (bind _returnvalue_3 (+ (`SceneComponent.K2_GetComponentLocation` (`self.StaticMesh`)) (0.0 -1020.0 0.0)))
  (bind _returnvalue_4 (+ (`SceneComponent.K2_GetComponentLocation` (`self.StaticMesh`)) (0.0 1000.0 0.0)))
  (bind _returnvalue_5 (+ (`SceneComponent.K2_GetComponentLocation` (`self.StaticMesh`)) (0.0 -1000.0 0.0)))
  (switch `int` (`KismetMathLibrary.RandomIntegerInRange` 0 4)
    (:`0`
      (`StaticMeshComponent.SetStaticMesh` (`self.StaticMesh`) "/Game/CR/Meshes/brightgrass.brightgrass")
      (for _index (range 12) :!label _label
        (if (< _dynspawn_y_2 1000.0)
          (if (>= _dynspawn_y_2 -1000.0)
            (switch `int` (`KismetMathLibrary.RandomIntegerInRange` 0 14)
              (:`0`
                (bind _returnvalue_6 (+ (* (`self.CurrentSpawn`) _index) (+ (`SceneComponent.K2_GetComponentLocation` (`self.StaticMesh`)) (`self.DynSpawn`))))
                (`|SpawnActorFromClass` "/Game/Blueprints/tree.tree_C" (`KismetMathLibrary.MakeTransform` _returnvalue_6) "Undefined" "OverrideRootScale" null null :!label _label_2))
              (:`1`
                (`|SpawnActorFromClass` "/Game/Blueprints/coin.coin_C" (`KismetMathLibrary.MakeTransform` _returnvalue_6) "Undefined" "OverrideRootScale" null null))
              (:`2`
                (goto _label_2))
              (:`3`
                (`|SpawnActorFromClass` "/Game/Blueprints/rock.rock_C" (`KismetMathLibrary.MakeTransform` _returnvalue_6) "Undefined" "OverrideRootScale" null null)))
            (set `self.CurrentSpawn` (+ (`self.CurrentSpawn`) (0.0 50.0 0.0)))
            (else
              (set `self.DynSpawn` (+ (`self.DynSpawn`) (`self.CurrentSpawn`)))))))
      (set `self.DynSpawn` (0.0 -600.0 0.0))
      (set `self.CurrentSpawn` (0.0 100.0 0.0)))
    (:`1`
      (`StaticMeshComponent.SetStaticMesh` (`self.StaticMesh`) "/Game/CR/Meshes/lightgrass.lightgrass")
      (goto _label))
    (:`2`
      (`StaticMeshComponent.SetStaticMesh` (`self.StaticMesh`) "/Game/CR/Materials/roadcenter.roadcenter")
      (switch `int` (`KismetMathLibrary.RandomIntegerInRange` 0 2)
        (:`0`
          (bind _returnvalue_7 (`|SpawnActorFromClass` "/Game/CR/Blueprints/Track.Track_C" (`KismetMathLibrary.MakeTransform` _returnvalue_5 (struct :`Yaw` 90.0)) "Undefined" "OverrideRootScale" null null))
          (bind _returnvalue_8 (`|SpawnActorFromClass` "/Game/CR/Blueprints/BlueCar.BlueCar_C" (`KismetMathLibrary.MakeTransform` _returnvalue_5) "Undefined" "OverrideRootScale" null null))
          (`/Game/CR/Blueprints/BlueCar.MoveCar` _returnvalue_8 _returnvalue_7))
        (:`1`
          (bind _returnvalue_9 (`|SpawnActorFromClass` "/Game/CR/Blueprints/Track.Track_C" (`KismetMathLibrary.MakeTransform` _returnvalue_4 (struct :`Yaw` 270.0)) "Undefined" "OverrideRootScale" null null))
          (bind _returnvalue_10 (`|SpawnActorFromClass` "/Game/CR/Blueprints/GreenCar.GreenCar_C" (`KismetMathLibrary.MakeTransform` _returnvalue_4) "Undefined" "OverrideRootScale" null null))
          (`/Game/CR/Blueprints/GreenCar.MoveCar` _returnvalue_10 _returnvalue_9))
        (:`2`
          (bind _returnvalue_11 (`|SpawnActorFromClass` "/Game/CR/Blueprints/Track.Track_C" (`KismetMathLibrary.MakeTransform` _returnvalue_3 (struct :`Yaw` 90.0)) "Undefined" "OverrideRootScale" null null))
          (bind _returnvalue_12 (`|SpawnActorFromClass` "/Game/CR/Blueprints/RedTruck.RedTruck_C" (`KismetMathLibrary.MakeTransform` _returnvalue_3) "Undefined" "OverrideRootScale" null null))
          (`/Game/CR/Blueprints/RedTruck.MoveCar` _returnvalue_12 _returnvalue_11))))
    (:`3`
      (`StaticMeshComponent.SetStaticMesh` (`self.StaticMesh`) "/Game/CR/Meshes/traintracks_nolight_.traintracks_nolight_")
      (bind _returnvalue_13 (`|SpawnActorFromClass` "/Game/CR/Blueprints/Track.Track_C" (`KismetMathLibrary.MakeTransform` _returnvalue_2 (struct :`Yaw` 270.0)) "Undefined" "OverrideRootScale" null null))
      (bind _returnvalue_14 (`|SpawnActorFromClass` "/Game/CR/Blueprints/Train.Train_C" (`KismetMathLibrary.MakeTransform` _returnvalue_2) "Undefined" "OverrideRootScale" null null))
      (`/Game/CR/Blueprints/Train.MoveCar` _returnvalue_14 _returnvalue_13))
    (:`4`
      (`StaticMeshComponent.SetStaticMesh` (`self.StaticMesh`) "/Game/CR/Meshes/water.water")
      (`|SpawnActorFromClass` "/Game/CR/Blueprints/WaterCollision.WaterCollision_C" (`KismetMathLibrary.MakeTransform` (`SceneComponent.K2_GetComponentLocation` (`self.StaticMesh`))) "Undefined" "OverrideRootScale" null null)
      (switch `int` (`KismetMathLibrary.RandomIntegerInRange` 0 1)
        (:`0`
          (for _index_2 (range 12)
            (if (< _dynspawn_y 600.0)
              (if (>= _dynspawn_y -700.0)
                (switch `int` (`KismetMathLibrary.RandomIntegerInRange` 0 6)
                  (:`0`
                    (bind _returnvalue_15 (+ (* (`self.CurrentSpawn`) _index_2) (+ (`SceneComponent.K2_GetComponentLocation` (`self.StaticMesh`)) (`self.DynSpawn`))))
                    (`|SpawnActorFromClass` "/Game/Blueprints/lilypad_pink.lilypad_pink_C" (`KismetMathLibrary.MakeTransform` _returnvalue_15) "Undefined" "OverrideRootScale" null null))
                  (:`1`
                    (`|SpawnActorFromClass` "/Game/Blueprints/lilypad_white.lilypad_white_C" (`KismetMathLibrary.MakeTransform` _returnvalue_15) "Undefined" "OverrideRootScale" null null))
                  (:`2`
                    (`|SpawnActorFromClass` "/Game/Blueprints/lilypad_green.lilypad_green_C" (`KismetMathLibrary.MakeTransform` _returnvalue_15) "Undefined" "OverrideRootScale" null null)))
                (set `self.CurrentSpawn` (+ (`self.CurrentSpawn`) (0.0 50.0 0.0)))
                (else
                  (set `self.DynSpawn` (+ (`self.DynSpawn`) (`self.CurrentSpawn`)))))))
          (set `self.DynSpawn` (0.0 -600.0 0.0))
          (set `self.CurrentSpawn` (0.0 100.0 0.0)))
        (:`1`
          (bind _returnvalue_16 (`|SpawnActorFromClass` "/Game/CR/Blueprints/Track.Track_C" (`KismetMathLibrary.MakeTransform` _returnvalue (struct :`Yaw` 270.0)) "Undefined" "OverrideRootScale" null null))
          (bind _returnvalue_17 (`|SpawnActorFromClass` "/Game/CR/Blueprints/Logs.Logs_C" (`KismetMathLibrary.MakeTransform` _returnvalue) "Undefined" "OverrideRootScale" null null))
          (`/Game/CR/Blueprints/Logs.MoveCar` _returnvalue_17 _returnvalue_16))))))

(fn `StartLevel`
  (for _ (range (+ (`KismetMathLibrary.RandomIntegerInRange` 3 4) 1))
    (`/Engine/EditorBlueprintResources/StandardMacros.IsValid` null
      (:`Is Valid`
        (`/Game/CR/Blueprints/BP_LevelSpawner.SpawnLevelAtSpawnPoint` (`self.LevelSpawner`))))))

(fn `UserConstructionScript`)