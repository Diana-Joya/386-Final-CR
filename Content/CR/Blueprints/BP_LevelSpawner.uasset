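; BP_LevelSpawner builds a chain of BP_Level segments at game start, each placed at the previous segment's SpawnPoint.
; BeginPlay spawns a short random batch, calling SetMesh only on its last segment, then a longer batch with SetMesh on each.
; Each segment receives a spawner reference; after startup, SpawnLevelAtSpawnPoint also calls SetMesh on the newest before extending.
; The first-segment fallback reads a BP_StartLevel cast that never executes.
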(event EventBeginPlay
  (CallFunction|SpawnInitialLevels)
  (Variables|Default|SetStartedGame true))

(event Collision|EventActorBeginOverlap
  (params (OtherActor :type Actor%20Object%20Reference)))

(event EventTick
  (params (DeltaSeconds :type Float%20%28single-precision%29)))

(fn ConstructionScript)

(fn SpawnLevel
  (params (SpawnLocation :type Vector))
  (bind _returnvalue (Game|SpawnActorfromClass "/Game/CR/Blueprints/BP_Level.BP_Level_C" (Math|Transform|MakeTransform SpawnLocation "0, 0, 0" "1,1,1") "Undefined" 0 0))
  (bind _output_get (Variables|Default|SetNewestLevel _returnvalue))
  (Variables|/Game/CR/Blueprints/BP_Level.BP_Level_C|SetLevelSpawner _output_get self))

(fn SpawnLevelatSpawnPoint
  (if (Variables|Default|GetStartedGame)
    (Default|SetMesh (Variables|Default|GetNewestLevel)))
  (CallFunction|SpawnLevel (Transformation|GetWorldLocation (Variables|/Game/CR/Blueprints/BP_Level.BP_Level_C|GetSpawnPoint (Variables|Default|GetNewestLevel)))))

(fn SpawnInitialLevels
  (for _index (range 1 (Math|Random|RandomIntegerinRange 3 4))
    (Utilities|IsValid (Variables|Default|GetNewestLevel)
      (:Is%20Valid
        (CallFunction|SpawnLevelatSpawnPoint))
      (:Is%20Not%20Valid
        (CallFunction|SpawnLevel (* (+ (Transformation|GetActorLocation (stale _asbp_start_level)) "60.000000, 0, 0") (Math|Vector|MakeVector (Math|Conversions|ToFloat(Integer) _index) 0.0 0.0))))))
  (Default|SetMesh (Variables|Default|GetNewestLevel))
  (CallFunction|SpawnNextLevels))

(fn SpawnNextLevels
  (for _index (range 1 (Math|Random|RandomIntegerinRange 17 20))
    (Utilities|IsValid (Variables|Default|GetNewestLevel)
      (:Is%20Valid
        (CallFunction|SpawnLevelatSpawnPoint))
      (:Is%20Not%20Valid
        (CallFunction|SpawnLevel (* (+ (Transformation|GetActorLocation (stale _asbp_start_level)) "60.000000, 0, 0") (Math|Vector|MakeVector (Math|Conversions|ToFloat(Integer) _index) 0.0 0.0)))))
    (Default|SetMesh (Variables|Default|GetNewestLevel)))
  (Default|SetMesh (Variables|Default|GetNewestLevel)))